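; Projectile bullet for the projectile weapon that damages rail paper targets and pushes physics objects on hit.
; On hit, it applies point damage to the target and adds a velocity-scaled impulse to simulating components.
; It briefly feeds the impact point to the target's AnimBP to curl the cloth, then clears it.
; The bullet destroys itself shortly afterwards, leaving time for that reset.
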(event `self.ReceiveHit`
  (params (MyComp :type "PrimitiveComponent Object Reference") (Other :type "Actor Object Reference") (OtherComp :type "PrimitiveComponent Object Reference") (bSelfMoved :type Boolean) (HitLocation :type "Vector Structure") (HitNormal :type "Vector Structure") (NormalImpulse :type "Vector Structure") (Hit :type "HitResult Structure (by ref)"))
  ;[1 0 0.007957] Handle Bullet Collisions with Targets and Physics Objects
  (`|ExecutionSequence`
    (:`then_0`
      (`self.TargetResponseToBullet` Hit))
    (:`then_1`
      (if (`SceneComponent.IsSimulatingPhysics` OtherComp "None")
        (`PrimitiveComponent.AddImpulseAtLocation` OtherComp (* (`self.GetVelocity`) (`self.WeaponDamage`)) (`self.K2_GetActorLocation`) "None")))
    (:`then_2`
      (`KismetSystemLibrary.Delay` 0.4)
      (`self.K2_DestroyActor`))))

(fn `UserConstructionScript`)
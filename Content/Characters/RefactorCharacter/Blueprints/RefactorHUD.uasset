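; RefactorHUD is the player HUD, creating the main HUD widget, raycast and projectile crosshairs, and a hidden end-game screen at BeginPlay.
; A bound crosshair-change event hides both crosshairs, then shows the one for the current weapon, though the initial selection uses a game-time variable.
; PushEndGameUI reveals the end screen and writes the current time to the game mode's RunningTime.
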(event `self.ReceiveBeginPlay`
  (bind _returnvalue (`GameplayStatics.GetPlayerController` 0))
  (`|ExecutionSequence`
    (:`then_0`
      ;[1 1 1] Create the UMG Widget and put on the players screen
      (bind _returnvalue_2 (`|CreateWidget` (`self.HUDType`) (`GameplayStatics.GetPlayerController` 0)))
      (bind _returnvalue_3 (`UserWidget.AddToPlayerScreen` _returnvalue_2 0))
      (if _returnvalue_3
        (set `self.HUDWidget` _returnvalue_2)))
    (:`then_1`
      ;[1 1 1] Create crosshairs
      (bind _returnvalue_4 (`|CreateWidget` (`self.RaycastUI`) _returnvalue))
      (bind _output_get (set `self.RaycastWidget` _returnvalue_4))
      (`UserWidget.AddToPlayerScreen` _output_get 0)
      (bind _returnvalue_5 (`|CreateWidget` (`self.ProjectileUI`) _returnvalue))
      (bind _output_get_2 (set `self.ProjectileWidget` _returnvalue_5))
      (`UserWidget.AddToPlayerScreen` _output_get_2 0)
      (`self.SetCurrentCrosshair` (`self.CUrrentGameTime`)))
    (:`then_2`
      ;[1 1 1] Create exit hud
      (bind _returnvalue_6 (`|CreateWidget` "/Game/Characters/RefactorCharacter/HUD/Exit_HUD.Exit_HUD_C"))
      (bind _output_get_3 (set `self.EndHUD` _returnvalue_6))
      (`UserWidget.AddToPlayerScreen` _output_get_3 0)
      (`Widget.SetVisibility` (`self.EndHUD`) "Hidden"))
    (:`then_3`
      ;[1 1 1] Change Texture
      (add `self.ChangeCrosshair` (delegate `ChangeCrosshair_Event`)))))

(event `ChangeCrosshair_Event` :!signature `self.ChangeCrosshair`
  (params (CurrentWeapon :type Integer))
  ;[1 1 1] Change Texture
  (`self.SetCurrentCrosshair` CurrentWeapon))

(event `PushEndGameUI`
  ;[1 1 1] End UI
  (`Widget.SetVisibility` (`self.EndHUD`) "Visible")
  (bind _frgamemode (`/Game/FiringRangeGame/BFL_FiringRangeHelpers.GetFRGameMode`))
  (set `/Game/FiringRangeGame/FiringRangeGameMode.RunningTime` (`GameplayStatics.GetTimeSeconds`) _frgamemode))

(fn `HideCurrentCrosshair`
  (`|ExecutionSequence`
    (:`then_0`
      (`Widget.SetVisibility` (`self.RaycastWidget`) "Hidden"))
    (:`then_1`
      (`Widget.SetVisibility` (`self.ProjectileWidget`) "Hidden"))))

(fn `SetCurrentCrosshair`
  (params (Selection :type Integer))
  (`self.HideCurrentCrosshair`)
  (switch `int` Selection
    (:`0`
      (`Widget.SetVisibility` (`self.RaycastWidget`) "Visible"))
    (:`1`
      (`Widget.SetVisibility` (`self.ProjectileWidget`) "Visible"))))

(fn `UpdateCurrentTime`
  (params (GameTime :type "Float (double-precision)"))
  (set `self.CurrentGameTime` (`KismetMathLibrary.FTrunc` GameTime)))

(fn `UserConstructionScript`)
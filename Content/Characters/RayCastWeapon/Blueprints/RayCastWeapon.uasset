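; Hitscan weapon that fires a visibility line trace along the camera aim and makes rail paper targets react to bullet hits.
; FireWeapon builds the ray from the camera, shifting its start toward the player's position along the shot direction.
; TargetResponseToBullet notifies the target, feeds the hit location to its anim Blueprint to curl the paper, then briefly delays before resetting it.
; The hit's collision UV places a bullet hole on the target's render target.
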(event `FireWeapon`
  (params (FireLocation :type "Vector Structure") (FireRotation :type "Rotator Structure") (PlayerLocation :type "Vector Structure") (PlayerRotation :type "Rotator Structure"))
  (bind _returnvalue (`KismetMathLibrary.Conv_RotatorToVector` FireRotation))
  (bind (_raystart _rayend) (`self.WeaponRayFromPlayer` FireLocation _returnvalue))
  ;[0 0.1406 1] Fire Bullet via Tracing and Respond to Targets
  (bind _outhit (`KismetSystemLibrary.LineTraceSingle` :`Start` (`self.WeaponFirePosAdjustment` PlayerLocation _raystart _returnvalue) :`End` _rayend :`TraceChannel` "TraceTypeQuery1" :`bTraceComplex` true :`DrawDebugType` "ForDuration" :`DrawTime` 2.0))
  (`self.TargetResponseToBullet` _outhit))

(fn `UserConstructionScript`)
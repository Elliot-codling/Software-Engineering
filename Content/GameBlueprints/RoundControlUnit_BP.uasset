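; Shooting range control unit with Up, Down and Start buttons that sets how many paper targets a round shows.
; Any detected trace starts the game mode's timer; Up and Down step the count within limits and update the text display.
; Start locks input, animates dynamic targets, reveals that many rail paper targets, then stores the game mode's calculated max hits in the global game state.
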(event `SetValues`
  ;[1 1 1] Set Initial Values on Play
  (`self.SetSpawnNo` (`self.MaxTargetsShown`)))

(event `OnTraceDetected`
  (params (Component :type "PrimitiveComponent Object Reference"))
  ;[1 1 1] Handle Interaction with Control Unit Buttons
  (bind _frgamemode (`/Game/FiringRangeGame/BFL_FiringRangeHelpers.GetFRGameMode`))
  (`/Game/FiringRangeGame/FiringRangeGameMode.StartGameTimer` _frgamemode)
  (if (`self.InputAllowed`)
    (if (== Component (`self.ButtonDown`))
      (`self.SetSpawnNo` (`self.DecrementSpawnNo`))
      (elif (== Component (`self.ButtonUp`))
        (`self.SetSpawnNo` (`self.IncrementSpawnNo`))
        (elif (== Component (`self.ButtonStart`))
          (set `self.InputAllowed` false)
          (bind _outactors (`GameplayStatics.GetAllActorsOfClass` "/Game/GameBlueprints/DynamicTarget_BP.DynamicTarget_BP_C"))
          (`/Game/GameBlueprints/DynamicTarget_BP.StartAnimation` _outactors)
          (bind _outactors_2 (`GameplayStatics.GetAllActorsOfClass` "/Game/GameBlueprints/RailPaperTarget_BP.RailPaperTarget_BP_C"))
          (for (_array_element _array_index) _outactors_2
            (`/Game/GameBlueprints/RailPaperTarget_BP.SetPaperVisibility` _array_element true)
            (if (>= _array_index (- (`self.NoTargetsShown`) 1))
              (break)))
          (bind _frgamemode_2 (`/Game/FiringRangeGame/BFL_FiringRangeHelpers.GetFRGameMode`))
          (bind _length (`/Game/FiringRangeGame/FiringRangeGameMode.CalculateMaxHits` _frgamemode_2))
          (bind _frglobalstate (`/Game/FiringRangeGame/BFL_FiringRangeHelpers.GetFRGLobalGameState`))
          (set `/Game/FiringRangeGame/FiringRangeGlobalState.MaxHits` _length _frglobalstate))))))

(fn `SetSpawnNo`
  (params (distance :type Integer))
  (bind _output_get (set `self.NoTargetsShown` distance))
  (`TextRenderComponent.K2_SetText` (`self.DefinedDistance`) (`KismetTextLibrary.Conv_IntToText` _output_get)))

(fn `UserConstructionScript`)
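; Spawner actor that places objects of a configurable class at random points inside its SpawnVolume bounds.
; BeginSpawn, which nothing in this Blueprint calls, starts a looping one-second timer that spawns an object and records it in SpawnedObstacles.
; Tick watches that array and calls EndSpawn to clear the timer once NumberToSpawn is reached.
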(event `self.ReceiveTick`
  (params (DeltaSeconds :type "Float (single-precision)"))
  (if (and (>= (`KismetArrayLibrary.Array_Length` (`self.SpawnedObstacles`)) (`self.NumberToSpawn`)) (`self.IsSpawning`))
    (`self.EndSpawn`)))

(event `SpawnAnObstacle`
  (bind (_origin _boxextent) (`KismetSystemLibrary.GetComponentBounds` (`self.SpawnVolume`)))
  ;[1 1 1] Spawn Object
  (bind _returnvalue (`|SpawnActorFromClass` (`self.ObjectType`) (`KismetMathLibrary.MakeTransform` (`KismetMathLibrary.RandomPointInBoundingBox` _origin _boxextent)) "Undefined" "MultiplyWithRoot" null null))
  (`KismetArrayLibrary.Array_Add` (`self.SpawnedObstacles`) _returnvalue))

(event `Begin Spawn`
  ;[1 1 1] Start Spawning
  (bind _returnvalue (`KismetSystemLibrary.K2_SetTimerDelegate` (delegate `SpawnAnObstacle`) 1.0 true))
  (set `self.TimerHandle` _returnvalue)
  (set `self.IsSpawning` true))

(event `EndSpawn`
  ;[1 1 1] End Spawning
  (`KismetSystemLibrary.K2_ClearAndInvalidateTimerHandle` (`self.TimerHandle`))
  (set `self.IsSpawning` false))

(fn `UserConstructionScript`)
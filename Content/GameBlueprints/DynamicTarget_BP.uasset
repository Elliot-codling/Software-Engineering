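; DynamicTarget_BP is a rail-mounted paper target actor that spawns and links its moving parts at BeginPlay.
; SpawnTargetSystem creates a RailPaperTarget_BP at the world origin and a RailTargetFollower_BP at the actor's location, setting the target as the follower's MovingActor.
; It then applies the cloth simulation setting and calls StartAnim, an empty event here, after a start delay.
; It also registers itself as OwningActor of its target status widget.
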(event `StartAnim`)

(event `self.ReceiveBeginPlay`
  (`|ExecutionSequence`
    (:`then_0`
      (`self.SpawnTargetSystem`)
      (set `SkeletalMeshComponent.bDisableClothSimulation` (not (`self.IsCloth`)) (`/Game/GameBlueprints/RailPaperTarget_BP.TargetPaper` (`self.Target`)))
      (`KismetSystemLibrary.Delay` (`self.StartDelay`))
      (`self.StartAnim`))
    (:`then_1`
      (bind _aswidget_target_status (cast `/Game/GameBlueprints/Widget_targetStatus` (`WidgetComponent.GetUserWidgetObject` (`self.TargetStatus`))))
      (set `/Game/GameBlueprints/Widget_targetStatus.OwningActor` self _aswidget_target_status))))

(fn `SpawnTargetSystem`
  (`|ExecutionSequence`
    (:`then_0`
      (bind _returnvalue (`|SpawnActorFromClass` "/Game/GameBlueprints/RailPaperTarget_BP.RailPaperTarget_BP_C" (`KismetMathLibrary.MakeTransform` (0.0 0.0 0.0)) "AlwaysSpawn" "MultiplyWithRoot" null null))
      (set `self.Target` _returnvalue))
    (:`then_1`
      (bind _returnvalue_2 (`|SpawnActorFromClass` "/Game/GameBlueprints/RailTargetFollower_BP.RailTargetFollower_BP_C" (`KismetMathLibrary.MakeTransform` (`self.K2_GetActorLocation`)) "Undefined" "MultiplyWithRoot" null null))
      (set `self.Follower` _returnvalue_2))
    (:`then_2`
      (set `/Game/GameBlueprints/RailTargetFollower_BP.MovingActor` (`self.Target`) (`self.Follower`)))))

(fn `UserConstructionScript`)
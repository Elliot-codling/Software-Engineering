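; A rail paper target that shows bullet holes where it is hit and tallies the hits.
; BeginPlay builds dynamic target and bullet-hole materials and a canvas render target, which it clears and feeds into the paper's texture parameter.
; CustomDrawHole stamps holes by passing the hit location to the hole material and drawing it to that render target.
; OnTargetHit increments the count and notifies the player's projectile or raycast character.
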(event `self.ReceiveBeginPlay`
  ;[1 1 1] Setup Materials for the Target Mesh
  (`|ExecutionSequence`
    (:`then_0`
      (bind _returnvalue (`PrimitiveComponent.CreateDynamicMaterialInstance` (`self.TargetPaper`) 0 "/Game/GameBlueprints/M_Target.M_Target" "None"))
      (set `self.TargetMaterial` _returnvalue))
    (:`then_1`
      (bind _returnvalue_2 (`KismetMaterialLibrary.CreateDynamicMaterialInstance` "/Game/GameBlueprints/M_BulletHole.M_BulletHole"))
      (set `self.BulletHoleMaterial` _returnvalue_2))
    (:`then_2`
      (bind _returnvalue_3 (`CanvasRenderTarget2D.CreateCanvasRenderTarget2D` "/Script/Engine.CanvasRenderTarget2D" (`self.RenderTargetWidth`) (`self.RenderTargetHeight`)))
      (set `self.RenderTarget` _returnvalue_3))
    (:`then_3`
      (`MaterialInstanceDynamic.SetTextureParameterValue` (`self.TargetMaterial`) (`self.TextureParam`) (`self.RenderTarget`))
      (`KismetRenderingLibrary.ClearRenderTarget2D` (`self.RenderTarget`)))))

(event `Event CustomDrawHole`
  (params (HoleLocation :type "Vector2D Structure"))
  ;[1 1 1] Dynamically Update BulletHole Material
  (`MaterialInstanceDynamic.SetVectorParameterValue` (`self.BulletHoleMaterial`) (`self.BulletHoleParam`) (`KismetMathLibrary.Conv_VectorToLinearColor` (`KismetMathLibrary.Conv_Vector2DToVector` HoleLocation)))
  (`KismetRenderingLibrary.DrawMaterialToRenderTarget` (`self.RenderTarget`) (`self.BulletHoleMaterial`)))

(event `OnTargetHit`
  (bind _returnvalue (`GameplayStatics.GetPlayerCharacter` 0))
  ;[1 1 1] Handle the tally on the number of hits
  (`/Engine/EditorBlueprintResources/StandardMacros.IncrementInt` (`self.NoHits`)
    (:`  `
      (bind _asprojectile_character (cast `/Game/Characters/ProjectileCharacter/Blueprints/ProjectileCharacter` _returnvalue)
        (:`then`
          (`/Game/Characters/ProjectileCharacter/Blueprints/ProjectileCharacter.HitTarget` _asprojectile_character 0))
        (:`CastFailed`
          (bind _asray_cast_character (cast `/Game/Characters/RayCastCharacter/Blueprints/RayCastCharacter` _returnvalue))
          (`/Game/Characters/RayCastCharacter/Blueprints/RayCastCharacter.HitTarget` _asray_cast_character 0))))))

(fn `UserConstructionScript`)
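; SpawnControlUnit_BP is an in-world control panel for setting how many items a linked Spawner spawns and starting it.
; It takes its initial count from the Spawner and shows the target on a text display.
; Traced hits on the up and down buttons adjust the count through clamp helpers.
; The start button passes the count to an idle Spawner, begins spawning and briefly locks input.
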(event `self.ReceiveBeginPlay`
  (bind _spawner (`self.Spawner`))
  ;[1 1 1] Set Initial Values on Play
  (`/Engine/EditorBlueprintResources/StandardMacros.IsValid` _spawner
    (:`Is Valid`
      (`self.SetSpawnNo` (`/Game/GameBlueprints/Spawner_BP.NumberToSpawn` _spawner)))))

(event `OnTraceDetected`
  (params (Component :type "PrimitiveComponent Object Reference"))
  (bind _spawner (`self.Spawner`))
  ;[1 1 1] Handle Interaction with Control Unit Buttons
  (if (`self.InputAllowed`)
    (if (== Component (`self.ButtonDown`))
      (`self.SetSpawnNo` (`self.DecrementSpawnNo`))
      (elif (== Component (`self.ButtonUp`))
        (`self.SetSpawnNo` (`self.IncrementSpawnNo`))
        (elif (== Component (`self.ButtonStart`))
          (if (not (`/Game/GameBlueprints/Spawner_BP.IsSpawning` (`self.Spawner`)))
            (set `/Game/GameBlueprints/Spawner_BP.NumberToSpawn` (`self.TargetSpawnNo`) _spawner)
            (`/Game/GameBlueprints/Spawner_BP.Begin Spawn` _spawner)
            (`self.AddInputDelay`)))))))

(fn `SetSpawnNo`
  (params (distance :type Integer))
  (bind _output_get (set `self.TargetSpawnNo` distance))
  (`TextRenderComponent.K2_SetText` (`self.DefinedDistance`) (`KismetTextLibrary.Conv_IntToText` _output_get)))

(fn `UserConstructionScript`)
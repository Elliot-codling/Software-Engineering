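; BP_DataReader is a tutorial actor that reads a DataTable and prints its contents to the screen.
; On BeginPlay it loops over every row name, looks up each row, and prints a formatted line for each row found.
; The format labels read Title, Score and Time, but they are fed from the row's DataName, Health and Damage fields.
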(event `self.ReceiveBeginPlay`
  (bind _data_table (`self.Data Table`))
  (bind _outrownames (`DataTableFunctionLibrary.GetDataTableRowNames` _data_table))
  (for _array_element _outrownames
    (bind _returnvalue (`|GetDataTableRow` _data_table _array_element)
      (:`then`
        (bind (_dataname _health _damage) (break `/Game/Tutorial_DataRead/Struct_Data` _returnvalue))
        (`KismetSystemLibrary.PrintString` (`KismetTextLibrary.Conv_TextToString` (`|FormatText` "Title: {Title} \nScore: {Score} \nTime: {Time}" (`KismetStringLibrary.Conv_NameToString` _dataname) (`KismetStringLibrary.Conv_DoubleToString` _health) (`KismetStringLibrary.Conv_DoubleToString` _damage))) true true (struct :`G` 0.66 :`B` 1.0 :`A` 1.0) 555.0)))))

(fn `UserConstructionScript`)